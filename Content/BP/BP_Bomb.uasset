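; BP_Bomb is a carryable bomb with a fuse that can be lit and put out.
; Pickup snaps it to the carrier's center-of-mass socket with collision off, while Drop detaches it in front of the carrier and restores collision.
; UsePrimary starts a looping one-second countdown that spawns an effect and destroys the bomb at zero.
; UseSecondary clears the ignited flag, so the loop resets the countdown on its next check.
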(event EventPickup
  (params (SkeletalMesh :type Skeletal%20Mesh%20Component%20Object%20Reference))
  (Transformation|AttachComponentToComponent SkeletalMesh "center_of_massSocket" "SnapToTarget" "SnapToTarget" "SnapToTarget" true)
  (Collision|SetCollisionEnabled (Variables|Default|GetBomb) "NoCollision"))

(event EventDrop
  (params (SkeletalMesh :type Skeletal%20Mesh%20Component%20Object%20Reference))
  (bind _returnvalue (Transformation|GetWorldTransform SkeletalMesh))
  (Development|PrintText "Drop Bomb")
  (Transformation|DetachFromActor "KeepRelative" "KeepRelative" "KeepRelative")
  (Transformation|SetActorTransform (Math|Transform|MakeTransform (+ (.location _returnvalue) (* (Math|Vector|GetForwardVector SkeletalMesh) 1e+02)) (.rotation _returnvalue) (.scale _returnvalue)))
  (Collision|SetCollisionEnabled (Variables|Default|GetBomb) "QueryAndPhysics"))

(event EventUsePrimary
  (Development|PrintText "Ignited Fuse")
  (Variables|Default|SetIgnited true)
  (if (> (Variables|Default|GetCountdown) 0) :!label _label
    (if (Variables|Default|GetIgnited)
      (bind _result (Math|Integer|DecrementInt (Variables|Default|GetCountdown))
        (:%20%20
          (bind _output_get (Variables|Default|SetCountdown _result))
          (Development|PrintText (Utilities|Text|ToText(Integer) _output_get) true true "(R=1.000000,G=0.000000,B=0.019647,A=1.000000)")
          (Utilities|FlowControl|Delay 1.0)
          (goto _label)))
      (else
        (Variables|Default|SetCountdown 5)))
    (else
      (Niagara|SpawnSystematLocation "/Game/VFX/CheckpointSystem.CheckpointSystem" (Transformation|GetWorldLocation (Variables|Default|GetBomb)))
      (Actor|DestroyActor))))

(event EventUseSecondary
  (Development|PrintText "Extinguished Fuse")
  (Variables|Default|SetIgnited false))

(fn ConstructionScript)