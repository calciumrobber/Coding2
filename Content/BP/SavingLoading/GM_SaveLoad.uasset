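; Game mode that saves and restores per-level world state and player stats through SaveGame objects.
; On BeginPlay it loads SG_LevelState from a slot named after the level and SG_PlayerStats from a shared slot, creating either if missing.
; Altered actors restore themselves via LoadStateMessage; stats and held item are applied to the third-person character.
; Separate save events write both objects; the per-type coin, door and key loaders are unused.
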(event Custom|SaveLevelStateToFile
  (bind _returnvalue (Game|GetCurrentLevelName true))
  (bind _returnvalue_2 (SaveGame|SaveGametoSlot (Variables|Default|GetSG_LevelState) _returnvalue))
  (if _returnvalue_2
    (Development|PrintText "Level State Saved!" true true "(R=0.000000,G=1.000000,B=0.052650,A=1.000000)" 3.0)
    (else
      (Development|PrintText "Level State Failed!" true true "(R=1.000000,G=0.025762,B=0.000000,A=1.000000)" 3.0))))

(event Custom|Load%20Level%20State%20From%20File
  (bind _returnvalue (Game|GetCurrentLevelName true))
  (bind _returnvalue_2 (SaveGame|DoesSaveGameExist _returnvalue))
  (if _returnvalue_2
    (bind _returnvalue_3 (SaveGame|LoadGamefromSlot _returnvalue))
    (bind _assg_level_state (Utilities|Casting|CastToSG_LevelState _returnvalue_3))
    (bind _output_get (Variables|Default|SetSG_LevelState _assg_level_state))
    (for _array_element (Variables|/Game/BP/SavingLoading/SG_LevelState.SG_LevelState_C|GetAlteredActors _output_get)
      (Class|BPILevelActorSaveable|LoadState(Message) _array_element))
    (else
      (bind _returnvalue_4 (SaveGame|CreateSaveGameObject "/Game/BP/SavingLoading/SG_LevelState.SG_LevelState_C"))
      (Variables|Default|SetSG_LevelState _returnvalue_4))))

(event Custom|SavePlayerStatsToFile
  (bind _returnvalue (SaveGame|SaveGametoSlot (Variables|Default|GetSG_PlayerStats) "PlayerSave"))
  (if _returnvalue
    (Development|PrintText "Player Stats Saved!" true true "(R=0.000000,G=1.000000,B=0.052650,A=1.000000)" 3.0)
    (else
      (Development|PrintText "Player Stats Failed!" true true "(R=1.000000,G=0.025762,B=0.000000,A=1.000000)" 3.0))))

(event Custom|LoadPlayerStatsFromFile
  (bind _returnvalue (SaveGame|DoesSaveGameExist "PlayerSave"))
  (if _returnvalue
    (bind _returnvalue_2 (SaveGame|LoadGamefromSlot "PlayerSave"))
    (bind _assg_player_stats (Utilities|Casting|CastToSG_PlayerStats _returnvalue_2))
    (bind _output_get (Variables|Default|SetSG_PlayerStats _assg_player_stats))
    (CallFunction|LoadPlayerStats _output_get)
    (else
      (bind _returnvalue_3 (SaveGame|CreateSaveGameObject "/Game/BP/SavingLoading/SG_PlayerStats.SG_PlayerStats_C"))
      (Variables|Default|SetSG_PlayerStats _returnvalue_3))))

(event EventBeginPlay
  (CallFunction|LoadLevelStatefromFile)
  (CallFunction|LoadPlayerStatsfromFile))

(fn ConstructionScript)

(fn LoadCollectedCoins
  (params (SG%20Level%20State :type SG%20Level%20State%20Object%20Reference))
  (for _array_element (Variables|/Game/BP/SavingLoading/SG_LevelState.SG_LevelState_C|GetCollectedCoins SG%20Level%20State)
    (Utilities|IsValid _array_element
      (:Is%20Valid
        (Default|CollectThyself _array_element)))))

(fn LoadOpenDoors
  (params (SG%20Level%20State :type SG%20Level%20State%20Object%20Reference))
  (for _array_element (Variables|/Game/BP/SavingLoading/SG_LevelState.SG_LevelState_C|GetDoorsUnlocked SG%20Level%20State)
    (Utilities|IsValid _array_element
      (:Is%20Valid
        (Default|UnlockThyself _array_element)))))

(fn LoadPlayerStats
  (params (SG%20PlayerStats :type SG%20Player%20Stats%20Object%20Reference))
  (bind _savehelditem (Variables|/Game/BP/SavingLoading/SG_PlayerStats.SG_PlayerStats_C|GetSaveHeldItem SG%20PlayerStats))
  (bind _asbp_third_person_character (Utilities|Casting|CastToBP_ThirdPersonCharacter (Game|GetPlayerCharacter 0)))
  (Variables|/Game/ThirdPerson/Blueprints/BP_ThirdPersonCharacter.BP_ThirdPersonCharacter_C|SetHealth _asbp_third_person_character (Variables|/Game/BP/SavingLoading/SG_PlayerStats.SG_PlayerStats_C|GetPlayerHealth SG%20PlayerStats))
  (Variables|/Game/ThirdPerson/Blueprints/BP_ThirdPersonCharacter.BP_ThirdPersonCharacter_C|SetMana _asbp_third_person_character (Variables|/Game/BP/SavingLoading/SG_PlayerStats.SG_PlayerStats_C|GetPlayerMana SG%20PlayerStats))
  (Variables|/Game/ThirdPerson/Blueprints/BP_ThirdPersonCharacter.BP_ThirdPersonCharacter_C|SetStamina _asbp_third_person_character (Variables|/Game/BP/SavingLoading/SG_PlayerStats.SG_PlayerStats_C|GetPlayerStamina SG%20PlayerStats))
  (Variables|/Game/ThirdPerson/Blueprints/BP_ThirdPersonCharacter.BP_ThirdPersonCharacter_C|SetTotalKeys _asbp_third_person_character (Variables|/Game/BP/SavingLoading/SG_PlayerStats.SG_PlayerStats_C|GetPlayerKeys SG%20PlayerStats))
  (Default|DebugStats _asbp_third_person_character)
  (Utilities|IsValid _savehelditem
    (:Is%20Valid
      (bind _output_get (Variables|/Game/ThirdPerson/Blueprints/BP_ThirdPersonCharacter.BP_ThirdPersonCharacter_C|SetHeldItem _asbp_third_person_character _savehelditem))
      (Class|BPIItem|Pickup(Message) _output_get (Variables|/Script/Engine.Character|GetMesh (Game|GetPlayerCharacter 0))))))

(fn LoadCollectedKeys
  (params (SG_LevelState :type SG%20Level%20State%20Object%20Reference))
  (for _array_element (Variables|/Game/BP/SavingLoading/SG_LevelState.SG_LevelState_C|GetCollectedKeys SG_LevelState)
    (Utilities|IsValid _array_element
      (:Is%20Valid
        (Default|CollectThyself _array_element)))))

(fn LoadCamDoors
  (params (SG%20Level%20State :type SG%20Level%20State%20Object%20Reference))
  (for _array_element (Variables|/Game/BP/SavingLoading/SG_LevelState.SG_LevelState_C|GetCameraDoorsUnlocked SG%20Level%20State)
    (Utilities|IsValid _array_element
      (:Is%20Valid
        (Default|LoadOpen _array_element)))))