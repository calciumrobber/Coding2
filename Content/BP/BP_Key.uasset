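; Collectible key pickup that bobs and spins through a Timeline started on BeginPlay.
; On overlap with BP_ThirdPersonCharacter it increments TotalKeys, adds itself to the GM_SaveLoad level state's AlteredActors, prints a placeholder for the pickup jingle and destroys itself.
; LoadState calls CollectThyself, which destroys the key without counting it again.
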(event OnComponentBeginOverlap(SM_Key)
  (params (OverlappedComponent :type Primitive%20Component%20Object%20Reference) (OtherActor :type Actor%20Object%20Reference) (OtherComp :type Primitive%20Component%20Object%20Reference) (OtherBodyIndex :type Integer) (bFromSweep :type Boolean) (SweepResult :type Hit%20Result%20Structure%20%28by%20ref%29))
  (bind _asbp_third_person_character (Utilities|Casting|CastToBP_ThirdPersonCharacter OtherActor))
  (bind _result (Math|Integer|IncrementInt (Variables|/Game/ThirdPerson/Blueprints/BP_ThirdPersonCharacter.BP_ThirdPersonCharacter_C|GetTotalKeys _asbp_third_person_character))
    (:%20%20
      (Variables|/Game/ThirdPerson/Blueprints/BP_ThirdPersonCharacter.BP_ThirdPersonCharacter_C|SetTotalKeys _asbp_third_person_character _result)
      (bind _asgm_save_load (Utilities|Casting|CastToGM_SaveLoad (Game|GetGameMode)))
      (Utilities|Array|AddUnique (Variables|/Game/BP/SavingLoading/SG_LevelState.SG_LevelState_C|GetAlteredActors (Variables|/Game/BP/SavingLoading/GM_SaveLoad.GM_SaveLoad_C|GetSG_LevelState _asgm_save_load)) self)
      (Development|PrintString "Insert Key Jingle Here")
      (Actor|DestroyActor))))

(event Custom|CollectThyself
  (Actor|DestroyActor))

(event EventBeginPlay
  (bind (_direction _float _spin) (Timeline|Timeline Play)
    (:Update
      (Transformation|SetRelativeLocationAndRotation (Variables|Default|GetSM_Key) (Math|Vector|MakeVector 0.0 0.0 (Math|Float|Lerp 1e+02 1.1e+02 _float)) (Math|Rotator|MakeRotator 0.0 0.0 (Math|Float|Lerp 0.0 3.6e+02 _spin)) false false))))

(event EventLoadState
  (CallFunction|CollectThyself))

(fn ConstructionScript)