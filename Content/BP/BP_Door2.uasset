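; BP_Door2 is a lockable swinging door that reacts to the third-person character entering its sphere trigger.
; If locked, it spends one of the character's keys and records itself in GM_SaveLoad's unlocked-door list before opening.
; A timeline rotates the door, reversing shortly after overlap ends, with DoOnce gating opening and FlipFlop toggling IsOpen on finish.
; UnlockThyself clears the lock without requiring a key.
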(event OnComponentBeginOverlap(Sphere)
  (params (OverlappedComponent :type Primitive%20Component%20Object%20Reference) (OtherActor :type Actor%20Object%20Reference) (OtherComp :type Primitive%20Component%20Object%20Reference) (OtherBodyIndex :type Integer) (bFromSweep :type Boolean) (SweepResult :type Hit%20Result%20Structure%20%28by%20ref%29))
  (bind _asbp_third_person_character (Utilities|Casting|CastToBP_ThirdPersonCharacter OtherActor))
  (if (Variables|Default|GetbIsLocked)
    (CallFunction|UnlockDoor)
    (else
      (CallFunction|OpenDoor))))

(event OnComponentEndOverlap(Sphere)
  (params (OverlappedComponent :type Primitive%20Component%20Object%20Reference) (OtherActor :type Actor%20Object%20Reference) (OtherComp :type Primitive%20Component%20Object%20Reference) (OtherBodyIndex :type Integer))
  (Utilities|Casting|CastToBP_ThirdPersonCharacter OtherActor)
  (Utilities|FlowControl|Delay 1.0)
  (CallFunction|CloseDoor))

(event Custom|UnlockDoor
  (if (> (Variables|/Game/ThirdPerson/Blueprints/BP_ThirdPersonCharacter.BP_ThirdPersonCharacter_C|GetTotalKeys (stale OnComponentBeginOverlap(Sphere) _asbp_third_person_character)) 0)
    (Development|PrintText "Unlocks Door" true true "(R=0.000000,G=1.000000,B=0.216170,A=1.000000)")
    (Variables|Default|SetbIsLocked false)
    (bind _result (Math|Integer|DecrementInt (Variables|/Game/ThirdPerson/Blueprints/BP_ThirdPersonCharacter.BP_ThirdPersonCharacter_C|GetTotalKeys (stale OnComponentBeginOverlap(Sphere) _asbp_third_person_character)))
      (:%20%20
        (Variables|/Game/ThirdPerson/Blueprints/BP_ThirdPersonCharacter.BP_ThirdPersonCharacter_C|SetTotalKeys (stale OnComponentBeginOverlap(Sphere) _asbp_third_person_character) _result)
        (bind _asgm_save_load (Utilities|Casting|CastToGM_SaveLoad (Game|GetGameMode)))
        (Utilities|Array|AddUnique (Variables|/Game/BP/SavingLoading/SG_LevelState.SG_LevelState_C|GetDoorsUnlocked (Variables|/Game/BP/SavingLoading/GM_SaveLoad.GM_SaveLoad_C|GetSG_LevelState _asgm_save_load)) self)
        (CallFunction|OpenDoor)))
    (else
      (Development|PrintText "Door is Locked"))))

(event Custom|OpenDoor
  (if (not (Variables|Default|GetbIsOpen))
    (Utilities|FlowControl|DoOnce false
      (:Completed
        (bind _newtrack_0 (Timeline|T_OpenDoor Play)
          (:Update
            (Transformation|SetRelativeRotation (Variables|Default|GetDoor) (Math|Rotator|MakeRotator 0.0 0.0 (Math|Float|Lerp 0.0 -9e+01 _newtrack_0)) false false))
          (:Finished
            (bind _isa (Utilities|FlowControl|FlipFlop)
              (:A
                _)
              (:B
                _))
            (bind _output_get (Variables|Default|SetbIsOpen _isa))
            (Development|PrintText (Utilities|Text|FormatText "bIsOpen = {bool}" _output_get))))))))

(event Custom|Close%20Door
  (if (Variables|Default|GetbIsOpen)
    (Utilities|FlowControl|Sequence
      (:then_0
        (bind _newtrack_0 (Timeline|T_OpenDoor Reverse)
          (:Update
            (Transformation|SetRelativeRotation (Variables|Default|GetDoor) (Math|Rotator|MakeRotator 0.0 0.0 (Math|Float|Lerp 0.0 -9e+01 _newtrack_0)) false false))
          (:Finished
            (bind _isa (Utilities|FlowControl|FlipFlop)
              (:A
                _)
              (:B
                _))
            (bind _output_get (Variables|Default|SetbIsOpen _isa))
            (Development|PrintText (Utilities|Text|FormatText "bIsOpen = {bool}" _output_get)))))
      (:then_1
        (Utilities|FlowControl|DoOnce false) ; enters at Reset
      ))))

(event Custom|UnlockThyself
  (Variables|Default|SetbIsLocked false))

(fn ConstructionScript)