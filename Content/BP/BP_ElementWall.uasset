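; An elemental barrier wall that only lets the player through when their element type matches the wall's element.
; On BeginPlay it picks the cube's material from the Element value and labels itself with a text render naming that barrier.
; A Box overlap disables the cube's collision for a matching BP_ThirdPersonCharacter and restores it whenever that character class leaves the box.
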(event OnComponentBeginOverlap(Box)
  (params (OverlappedComponent :type Primitive%20Component%20Object%20Reference) (OtherActor :type Actor%20Object%20Reference) (OtherComp :type Primitive%20Component%20Object%20Reference) (OtherBodyIndex :type Integer) (bFromSweep :type Boolean) (SweepResult :type Hit%20Result%20Structure%20%28by%20ref%29))
  (bind _asbp_third_person_character (Utilities|Casting|CastToBP_ThirdPersonCharacter OtherActor))
  (if (Utilities|Enum|Equal(Enum) (Variables|/Game/ThirdPerson/Blueprints/BP_ThirdPersonCharacter.BP_ThirdPersonCharacter_C|GetElementType _asbp_third_person_character) (Variables|Default|GetElement))
    (Collision|SetCollisionEnabled (Variables|Default|GetCube) "NoCollision")))

(event OnComponentEndOverlap(Box)
  (params (OverlappedComponent :type Primitive%20Component%20Object%20Reference) (OtherActor :type Actor%20Object%20Reference) (OtherComp :type Primitive%20Component%20Object%20Reference) (OtherBodyIndex :type Integer))
  (Utilities|Casting|CastToBP_ThirdPersonCharacter OtherActor)
  (Collision|SetCollisionEnabled (Variables|Default|GetCube) "QueryAndPhysics"))

(event EventBeginPlay
  (bind _element (Variables|Default|GetElement))
  (Rendering|Material|SetMaterial (Variables|Default|GetCube) 0 (Utilities|Select :Index _element :NewEnumerator0 "/Game/Materials/MI_Default.MI_Default" :NewEnumerator1 "/Game/Materials/MI_FlatBlack.MI_FlatBlack" :NewEnumerator2 "/Game/Materials/MI_FlatRed.MI_FlatRed" :NewEnumerator3 "/Game/Materials/MI_Ice.MI_Ice" :NewEnumerator4 "/Game/Materials/MI_FlatYellow.MI_FlatYellow" :NewEnumerator5 "/Game/Materials/MI_Radiant.MI_Radiant"))
  (Rendering|Components|TextRender|SetText (Variables|Default|GetTextRender) (Utilities|Text|FormatText "{element} Barrier" (|GenerictoText _element))))

(fn ConstructionScript)