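; BP_SpawnEnemyManager is a manager actor that populates the level with randomized AI enemies on BeginPlay.
; It gathers every BP_EnemySpawnPoint, prints their count, and gives each a 75% chance to spawn a BP_AiMoveTo at its transform, owned by that point.
; Each spawned enemy gets a random skeletal mesh, name text, and independently picked materials for its first two slots from the manager's arrays.
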(event EventBeginPlay
  (bind _material (Variables|Default|GetMaterial))
  (bind _outactors (Actor|GetAllActorsOfClass "/Game/BP/BP_EnemySpawnPoint.BP_EnemySpawnPoint_C"))
  (Development|PrintText (Utilities|Text|FormatText "There are {index} spawn points." (Utilities|Array|Length _outactors)))
  (for _array_element _outactors
    (if (Math|Random|RandomBoolwithWeight 0.75)
      (bind _returnvalue (Game|SpawnActorfromClass "/Game/AI_Blueprints/BP_AiMoveTo.BP_AiMoveTo_C" (Transformation|GetActorTransform _array_element) "Undefined" "MultiplyWithRoot" _array_element 0))
      (Components|SkeletalMesh|SetSkeletalMeshAsset (Variables|/Script/Engine.Character|GetMesh _returnvalue) (.OutItem (Utilities|Array|Random (Variables|Default|GetSkeletalMesh))))
      (Rendering|Components|TextRender|SetText (Variables|/Game/AI_Blueprints/BP_AiMoveTo.BP_AiMoveTo_C|Getai%20Name%20Text _returnvalue) (.OutItem (Utilities|Array|Random (Variables|Default|GetNames))))
      (Rendering|Material|SetMaterial (Variables|/Script/Engine.Character|GetMesh _returnvalue) 0 (.OutItem (Utilities|Array|Random _material)))
      (Rendering|Material|SetMaterial (Variables|/Script/Engine.Character|GetMesh _returnvalue) 1 (.OutItem (Utilities|Array|Random _material))))))

(fn ConstructionScript)