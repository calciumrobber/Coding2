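; BP_ElementBracelet is a pickup item that attaches to the right-hand IK socket and temporarily changes the player's element.
; Primary use overrides the third-person character's ElementType for a five-second delay-loop countdown, then restores it, refusing reuse while running.
; Secondary use cycles the bracelet element, updating the cylinder material and debug text.
; The modulo-5 cycle never selects Radiant, the sixth option.
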(event EventPickup
  (params (SkeletalMesh :type Skeletal%20Mesh%20Component%20Object%20Reference))
  (Transformation|AttachComponentToComponent SkeletalMesh "ik_hand_r" "SnapToTarget" "SnapToTarget" "SnapToTarget" true)
  (Collision|SetCollisionEnabled (Variables|Default|GetCylinder) "NoCollision"))

(event EventDrop
  (params (SkeletalMesh :type Skeletal%20Mesh%20Component%20Object%20Reference))
  (Development|PrintText "Drop Flashlight")
  (Transformation|DetachFromActor "KeepRelative" "KeepRelative" "KeepRelative")
  (Transformation|SetActorTransform (Transformation|GetWorldTransform SkeletalMesh))
  (Collision|SetCollisionEnabled (Variables|Default|GetCylinder) "QueryAndPhysics"))

(event EventUseSecondary
  (Variables|Default|SetElementIndex (Math|Integer|%(Integer) (+ (Variables|Default|GetElementIndex) 1) 5))
  (Variables|Default|SetBraceletElement (Utilities|Select :Index (Variables|Default|GetElementIndex) :Option%200 "NewEnumerator0" :Option%201 "NewEnumerator1" :Option%202 "NewEnumerator2" :Option%203 "NewEnumerator3" :Option%204 "NewEnumerator4" :Option%205 "NewEnumerator5"))
  (Rendering|Material|SetMaterial (Variables|Default|GetCylinder) 0 (Utilities|Select :Index (Variables|Default|GetBraceletElement) :NewEnumerator0 "/Game/Materials/MI_Default.MI_Default" :NewEnumerator1 "/Game/Materials/MI_FlatBlack.MI_FlatBlack" :NewEnumerator2 "/Game/Materials/MI_FlatRed.MI_FlatRed" :NewEnumerator3 "/Game/Materials/MI_Ice.MI_Ice" :NewEnumerator4 "/Game/Materials/MI_FlatYellow.MI_FlatYellow" :NewEnumerator5 "/Game/Materials/MI_Radiant.MI_Radiant"))
  (Development|PrintText (Utilities|Text|FormatText "{element} {index}" (|GenerictoText (Variables|Default|GetBraceletElement)) (Variables|Default|GetElementIndex))))

(event EventUsePrimary
  (if (== (Variables|Default|GetCountdown) 5)
    (bind _asbp_third_person_character (Utilities|Casting|CastToBP_ThirdPersonCharacter (Game|Player|GetPlayerPawn 0)))
    (Variables|Default|SetOldElement (Variables|/Game/ThirdPerson/Blueprints/BP_ThirdPersonCharacter.BP_ThirdPersonCharacter_C|GetElementType _asbp_third_person_character))
    (Variables|/Game/ThirdPerson/Blueprints/BP_ThirdPersonCharacter.BP_ThirdPersonCharacter_C|SetElementType _asbp_third_person_character (Variables|Default|GetBraceletElement))
    (if (> (Variables|Default|GetCountdown) 0) :!label _label
      (Development|PrintText (Utilities|Text|ToText(Integer) (Variables|Default|GetCountdown)))
      (bind _result (Math|Integer|DecrementInt (Variables|Default|GetCountdown))
        (:%20%20
          (Variables|Default|SetCountdown _result)
          (Utilities|FlowControl|Delay 1.0)
          (goto _label)))
      (else
        (Variables|/Game/ThirdPerson/Blueprints/BP_ThirdPersonCharacter.BP_ThirdPersonCharacter_C|SetElementType _asbp_third_person_character (Variables|Default|GetOldElement))
        (Variables|Default|SetCountdown 5)))
    (else
      (Development|PrintText "Bracelet already running"))))

(event EventBeginPlay
  (Variables|Default|SetBraceletElement (Utilities|Select :Index (Variables|Default|GetElementIndex) :Option%200 "NewEnumerator0" :Option%201 "NewEnumerator1" :Option%202 "NewEnumerator2" :Option%203 "NewEnumerator3" :Option%204 "NewEnumerator4" :Option%205 "NewEnumerator5"))
  (Rendering|Material|SetMaterial (Variables|Default|GetCylinder) 0 (Utilities|Select :Index (Variables|Default|GetBraceletElement) :NewEnumerator0 "/Game/Materials/MI_Default.MI_Default" :NewEnumerator1 "/Game/Materials/MI_FlatBlack.MI_FlatBlack" :NewEnumerator2 "/Game/Materials/MI_FlatRed.MI_FlatRed" :NewEnumerator3 "/Game/Materials/MI_Ice.MI_Ice" :NewEnumerator4 "/Game/Materials/MI_FlatYellow.MI_FlatYellow" :NewEnumerator5 "/Game/Materials/MI_Radiant.MI_Radiant"))
  (Development|PrintText (Utilities|Text|FormatText "{element} {index}" (|GenerictoText (Variables|Default|GetBraceletElement)) (Variables|Default|GetElementIndex))))

(fn ConstructionScript)