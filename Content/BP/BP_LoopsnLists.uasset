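; BP_LoopsnLists is a demo Blueprint that shows loop and array techniques through colored on-screen text.
; Separate custom events demonstrate a countdown While loop that resets its counter, an indexed For loop, and a ForEach over an array of colors.
; DelayLoop re-calls itself through a Delay and a DoN limit, also triggering the For loop each pass.
; BeginPlay is empty, so nothing in this Blueprint starts the demos.
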(event Custom|DelayLoop
  (Development|PrintText (Utilities|Text|FormatText "This has run  {count} times." (stale _counter)))
  (Utilities|FlowControl|Delay 0.1)
  (bind _counter (Utilities|FlowControl|DoN 20)
    (:Exit
      (CallFunction|StartforLoop)
      (CallFunction|DelayLoop))))

(event Custom|StartForLoop
  (bind _array (Utilities|Array|MakeArray "(R=1.000000,G=0.000886,B=0.243511,A=1.000000)" "(R=1.000000,G=0.000000,B=0.029683,A=1.000000)" "(R=1.000000,G=0.339692,B=0.000000,A=1.000000)" "(R=1.000000,G=0.885046,B=0.000000,A=1.000000)" "(R=0.631435,G=1.000000,B=0.000000,A=1.000000)" "(R=0.352714,G=1.000000,B=0.000000,A=1.000000)"))
  (for _index (range 0 (- (Utilities|Array|Length _array) 1) 2)
    (Development|PrintText (Utilities|Text|FormatText "This is index # {index}." _index) true true (Utilities|Array|Get(acopy) _array _index))))

(event Custom|StartWhileLoop
  (while (> (Variables|Default|GetWhileLoopCounter) 0)
    (Development|PrintText (Utilities|Text|FormatText "There are {uses} left." (Variables|Default|GetWhileLoopCounter)) true true "(R=0.005810,G=1.000000,B=0.303005,A=1.000000)")
    (bind _result (Math|Integer|DecrementInt (Variables|Default|GetWhileLoopCounter))
      (:%20%20
        (Variables|Default|SetWhileLoopCounter _result))))
  (Variables|Default|SetWhileLoopCounter 10))

(event Custom|StartForEachLoop
  (for (_array_element _array_index) (Utilities|Array|MakeArray "(R=1.000000,G=0.000886,B=0.243511,A=1.000000)" "(R=1.000000,G=0.000000,B=0.029683,A=1.000000)" "(R=1.000000,G=0.339692,B=0.000000,A=1.000000)" "(R=1.000000,G=0.885046,B=0.000000,A=1.000000)" "(R=0.631435,G=1.000000,B=0.000000,A=1.000000)" "(R=0.352714,G=1.000000,B=0.000000,A=1.000000)")
    (Development|PrintText (Utilities|Text|FormatText "For Each {index}" _array_index) true true _array_element)))

(event EventBeginPlay)

(fn ConstructionScript)