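; BP_Door is a lockable swinging door that responds when the third-person character overlaps its sphere.
; If locked, it spends one of the character's keys to unlock without opening, or plays a short rattle timeline without keys.
; If unlocked, a DoOnce-gated timeline swings the mesh open, then reverses after a delay on exit, with FlipFlop tracking open state.
; Sounds are PrintString placeholders, and the save/load game mode cast leads nowhere.
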(event OnComponentBeginOverlap(Sphere)
  (params (OverlappedComponent :type Primitive%20Component%20Object%20Reference) (OtherActor :type Actor%20Object%20Reference) (OtherComp :type Primitive%20Component%20Object%20Reference) (OtherBodyIndex :type Integer) (bFromSweep :type Boolean) (SweepResult :type Hit%20Result%20Structure%20%28by%20ref%29))
  (bind _asbp_third_person_character (Utilities|Casting|CastToBP_ThirdPersonCharacter OtherActor))
  (if (Variables|Default|GetisDoorLocked) ; Check if Door is Locked
    ;[0.15 0.15 0.15 0.5] ifDoorLocked=true
    (if (> (Variables|/Game/ThirdPerson/Blueprints/BP_ThirdPersonCharacter.BP_ThirdPersonCharacter_C|GetTotalKeys _asbp_third_person_character) 0)
      (Development|PrintString "Insert Unlock Sound Here") ; Unlock Door
      (Variables|Default|SetisDoorLocked false)
      (bind _result (Math|Integer|DecrementInt (Variables|/Game/ThirdPerson/Blueprints/BP_ThirdPersonCharacter.BP_ThirdPersonCharacter_C|GetTotalKeys _asbp_third_person_character))
        (:%20%20
          (Variables|/Game/ThirdPerson/Blueprints/BP_ThirdPersonCharacter.BP_ThirdPersonCharacter_C|SetTotalKeys _asbp_third_person_character _result)
          (Utilities|FlowControl|Delay 0.2)
          (Utilities|Casting|CastToGM_SaveLoad (Game|GetGameMode))))
      (else
        (bind _newtrack_1 (Timeline|DoorLocked PlayFromStart) ; Rattle Door if no keys
          (:Update
            (Transformation|SetRelativeRotation (Variables|Default|GetSM_Door) (Math|Rotator|MakeRotator 0.0 0.0 (Math|Float|Lerp 0.0 -5.0 _newtrack_1)) false false))
          (:Finished
            (Development|PrintString "Insert Door Rattle Sound Here")))))
    (else
      ;[0.15 0.15 0.15 0.5] ifDoorLocked=false
      (if (not (Variables|Default|GetisDoorOpen))
        (Utilities|FlowControl|DoOnce false
          (:Completed
            (Development|PrintString "Insert Door Open Sound Here")
            (bind _dooropen (Timeline|Timeline Play)
              (:Update
                (Transformation|SetRelativeRotation (Variables|Default|GetSM_Door) (Math|Rotator|MakeRotator 0.0 0.0 (Math|Float|Lerp 0.0 -9e+01 _dooropen)) false false))
              (:Finished
                (bind _isa (Utilities|FlowControl|FlipFlop)
                  (:A
                    _)
                  (:B
                    _))
                (Variables|Default|SetisDoorOpen _isa)))))))))

(event OnComponentEndOverlap(Sphere)
  (params (OverlappedComponent :type Primitive%20Component%20Object%20Reference) (OtherActor :type Actor%20Object%20Reference) (OtherComp :type Primitive%20Component%20Object%20Reference) (OtherBodyIndex :type Integer))
  (Utilities|Casting|CastToBP_ThirdPersonCharacter OtherActor)
  (Utilities|FlowControl|Delay 1.0)
  (if (Variables|Default|GetisDoorOpen)
    (Utilities|FlowControl|Sequence
      (:then_0
        (Development|PrintString "Insert Door Close Sound here")
        ;[0.15 0.15 0.15 0.5] ifDoorLocked=false
        (bind _dooropen (Timeline|Timeline ReverseFromEnd)
          (:Update
            (Transformation|SetRelativeRotation (Variables|Default|GetSM_Door) (Math|Rotator|MakeRotator 0.0 0.0 (Math|Float|Lerp 0.0 -9e+01 _dooropen)) false false))
          (:Finished
            (bind _isa (Utilities|FlowControl|FlipFlop)
              (:A
                _)
              (:B
                _))
            (Variables|Default|SetisDoorOpen _isa))))
      (:then_1
        (Utilities|FlowControl|DoOnce false) ; enters at Reset
      ))))

(fn ConstructionScript)