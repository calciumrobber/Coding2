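; BP_EnemyBase is an enemy character Blueprint providing attack, aggro, walk speed and patrol functions.
; Attack plays a left-hook montage and calls the AttackFinished dispatcher on completion or interruption.
; Aggro events set a flag and swap a mesh material to flat red, restoring the original cached at BeginPlay.
; Patrol lookup steps along the route's spline points, reversing direction at the bounds to ping-pong.
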(event Custom|Attack
  (Development|PrintText "Get shanked")
  (Animation|Montage|PlayMontage (Variables|Character|GetMesh) "/Game/CloseCombatAnimSet/Animations/InPlace/Attacks/NinjaLeftHook_Montage.NinjaLeftHook_Montage"
    (:OnCompleted
      _)
    (:OnInterrupted
      _))
  (Default|CallAttackFinished))

(event Custom|GetAggroed
  (Rendering|Material|SetMaterial (Variables|Character|GetMesh) 1 "/Game/Materials/MI_FlatRed.MI_FlatRed")
  (Variables|Default|SetbIsAggroed true))

(event Custom|LoseAggro
  (Rendering|Material|SetMaterial (Variables|Character|GetMesh) 1 (Variables|Default|GetOriginalMaterial))
  (Variables|Default|SetbIsAggroed false))

(event Custom|SetWalkSpeed
  (params (Max%20Walk%20Speed :type Float%20%28single-precision%29))
  (Variables|/Script/Engine.CharacterMovementComponent|SetMaxWalkSpeed (Variables|Character|GetCharacterMovement) Max%20Walk%20Speed))

(event EventBeginPlay
  (Variables|Default|SetOriginalMaterial (Rendering|Material|GetMaterial (Variables|Character|GetMesh) 1)))

(fn ConstructionScript)

(fn GetPatrolPointLocation
  (Variables|Default|SetPatrolIndex (+ (Variables|Default|GetPatrolIndex) (Variables|Default|GetDirection)))
  (if (or (<= (Variables|Default|GetPatrolIndex) 0) (>= (Variables|Default|GetPatrolIndex) (Spline|GetNumberOfSplinePoints (Variables|/Game/AI_Blueprints/NewAI/BP_PatrolRoute.BP_PatrolRoute_C|GetSpline (Variables|Default|GetPatrolRoute)))))
    (Variables|Default|SetDirection (* (Variables|Default|GetDirection) -1)))
  (return (Spline|GetLocationatSplinePoint (Variables|/Game/AI_Blueprints/NewAI/BP_PatrolRoute.BP_PatrolRoute_C|GetSpline (Variables|Default|GetPatrolRoute)) (Variables|Default|GetPatrolIndex) "World")))