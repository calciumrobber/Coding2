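; BP_PatrolRoute defines a patrol path with a spline and supplies successive world-space patrol locations, presumably for AI.
; Each GetPatrolPointLocation call steps PatrolIndex by Direction and returns that spline point's location.
; Direction flips when the index reaches zero or the point count, so the route ping-pongs instead of looping.
; The upper check uses the point count rather than the last valid index, so the index steps one past the end.
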(fn ConstructionScript)

(fn GetPatrolPointLocation
  (Variables|Default|SetPatrolIndex (+ (Variables|Default|GetPatrolIndex) (Variables|Default|GetDirection)))
  (if (or (<= (Variables|Default|GetPatrolIndex) 0) (>= (Variables|Default|GetPatrolIndex) (Spline|GetNumberOfSplinePoints (Variables|Default|GetSpline))))
    (Variables|Default|SetDirection (* (Variables|Default|GetDirection) -1)))
  (return (Spline|GetLocationatSplinePoint (Variables|Default|GetSpline) (Variables|Default|GetPatrolIndex) "World")))