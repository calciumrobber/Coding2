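; BP_CamDoorTrigger is a one-shot trigger that opens its Target door when the player character walks into its sphere.
; On overlap it passes the player to OpenDoor, noted as the new view target.
; It then registers Target in the GM_SaveLoad game mode's level-state AlteredActors for saving and destroys the sphere component, provided that game mode cast succeeds.
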(event OnComponentBeginOverlap(Sphere1)
  (params (OverlappedComponent :type Primitive%20Component%20Object%20Reference) (OtherActor :type Actor%20Object%20Reference) (OtherComp :type Primitive%20Component%20Object%20Reference) (OtherBodyIndex :type Integer) (bFromSweep :type Boolean) (SweepResult :type Hit%20Result%20Structure%20%28by%20ref%29))
  (Utilities|Casting|CastToBP_ThirdPersonCharacter OtherActor)
  (Default|OpenDoor (Variables|Default|GetTarget) OtherActor) ; new view target is the player
  (bind _asgm_save_load (Utilities|Casting|CastToGM_SaveLoad (Game|GetGameMode)))
  (Utilities|Array|AddUnique (Variables|/Game/BP/SavingLoading/SG_LevelState.SG_LevelState_C|GetAlteredActors (Variables|/Game/BP/SavingLoading/GM_SaveLoad.GM_SaveLoad_C|GetSG_LevelState _asgm_save_load)) (Variables|Default|GetTarget))
  (Components|DestroyComponent (Variables|Default|GetSphere1)))

(event EventBeginPlay)

(event Collision|EventActorBeginOverlap
  (params (OtherActor :type Actor%20Object%20Reference)))

(event EventTick
  (params (DeltaSeconds :type Float%20%28single-precision%29)))

(fn ConstructionScript)